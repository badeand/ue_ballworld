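; BP_OSCBall is a physics ball actor meant to be driven by OSC messages.
; Each tick pushes the sphere along world Y and Z using ForceX and ForceY.
; An OSC receiver event feeds address-suffix handlers for scaled X/Y forces, hide/show and material BaseColor from RGB values.
; As wired, each handler compares the address to itself plus its suffix, so those branches cannot match.
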(event `self.ReceiveTick`
  (params (DeltaSeconds :type "Float (single-precision)"))
  (`PrimitiveComponent.AddForce` (`self.Sphere`) (`KismetMathLibrary.MakeVector` 0.0 (`self.ForceX`) (`self.ForceY`)) "None" false))

(event `self.OscReceiverComponent.OnOscReceived`
  (params (Address :type "Name (by ref)") (Data :type "Array of OscDataElemStruct Structure (by ref)") (SenderIp :type String))
  (bind (_output _value) (`OscFunctionLibrary.PopFloat` Data))
  (bind _returnvalue (`KismetStringLibrary.Conv_NameToString` (`self.Address`)))
  (bind (_output_2 _value_2) (`OscFunctionLibrary.PopFloat` _output))
  (`|ExecutionSequence`
    (:`then_0`
      (if (`KismetStringLibrary.EqualEqual_StrStr` (`KismetStringLibrary.Conv_NameToString` Address) (`KismetStringLibrary.Concat_StrStr` _returnvalue "/x"))
        (set `self.ForceX` (* (* (- (`.Value` (`OscFunctionLibrary.PopFloat` Data)) 0.5) -1.0) 20000.0))))
    (:`then_1`
      (if (`KismetStringLibrary.EqualEqual_StrStr` (`KismetStringLibrary.Conv_NameToString` Address) (`KismetStringLibrary.Concat_StrStr` _returnvalue "/y"))
        (set `self.ForceY` (* (`KismetMathLibrary.FMin` (* (- (`.Value` (`OscFunctionLibrary.PopFloat` Data)) 0.5) -1.0)) 100000.0))))
    (:`then_2`
      (if (`KismetStringLibrary.EqualEqual_StrStr` (`KismetStringLibrary.Conv_NameToString` Address) (`KismetStringLibrary.Concat_StrStr` _returnvalue "/remove"))
        (`self.SetActorHiddenInGame` true)))
    (:`then_3`
      (if (`KismetStringLibrary.EqualEqual_StrStr` (`KismetStringLibrary.Conv_NameToString` Address) (`KismetStringLibrary.Concat_StrStr` _returnvalue "/add"))
        (`self.SetActorHiddenInGame` false)))
    (:`then_4`
      (if (`KismetStringLibrary.EqualEqual_StrStr` (`KismetStringLibrary.Conv_NameToString` Address) (`KismetStringLibrary.Concat_StrStr` _returnvalue "/color"))
        (`MeshComponent.SetVectorParameterValueOnMaterials` (`self.Sphere`) "BaseColor" (`KismetMathLibrary.MakeVector` (/ _value 255.0) (/ _value_2 255.0) (/ (`.Value` (`OscFunctionLibrary.PopFloat` _output_2)) 255.0)))))))

(fn `CreateVector`
  (params (input :type "Array of OscDataElemStruct Structure (by ref)"))
  (returns (ReturnValue :type "Vector Structure"))
  (bind (_output _value) (`OscFunctionLibrary.PopFloat` input))
  (bind (_output_2 _value_2) (`OscFunctionLibrary.PopFloat` _output))
  (return (`KismetMathLibrary.MakeVector` _value _value_2 (`.Value` (`OscFunctionLibrary.PopFloat` _output_2)))))

(fn `UserConstructionScript`)